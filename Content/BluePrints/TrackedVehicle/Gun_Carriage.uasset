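; Gun carriage actor for a tracked vehicle, carrying a battery of four guns gathered into GunsCollection at construction.
; TargetGuns turns each gun toward a target in the actor's local space, clamped to a limited pitch and side-facing yaw arc.
; FireGuns fires all four after short random delays, each spawning a projectile at its Muzzle socket with slight rotation and speed variation, then applying a recoil impulse.
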(event `self.ReceiveTick`
  (params (DeltaSeconds :type "Float (single-precision)")))

(event `/Game/BluePrints/Interfaces/WeaponsController.FireGuns`
  (`|ExecutionSequence`
    (:`then_0`
      (`KismetSystemLibrary.Delay` (`KismetMathLibrary.RandomFloatInRange` 0.0 0.3))
      (`self.FireGun` (`|GetArrayItem` (`self.Guns_Collection`))))
    (:`then_1`
      (`KismetSystemLibrary.Delay` (`KismetMathLibrary.RandomFloatInRange` 0.0 0.3))
      (`self.FireGun` (`|GetArrayItem` (`self.Guns_Collection`) 1)))
    (:`then_2`
      (`KismetSystemLibrary.Delay` (`KismetMathLibrary.RandomFloatInRange` 0.0 0.3))
      (`self.FireGun` (`|GetArrayItem` (`self.Guns_Collection`) 2)))
    (:`then_3`
      (`KismetSystemLibrary.Delay` (`KismetMathLibrary.RandomFloatInRange` 0.0 0.3))
      (`self.FireGun` (`|GetArrayItem` (`self.Guns_Collection`) 3)))))

(event `/Game/BluePrints/Interfaces/WeaponsController.TargetGuns`
  (params (Target :type "Vector Structure"))
  (for _array_element (`self.Guns_Collection`)
    (`self.AllignGun` Target _array_element)))

(fn `AllignGun`
  (params (Target :type "Vector Structure") (Gun :type "StaticMeshComponent Object Reference"))
  (bind _returnvalue_location (`KismetMathLibrary.BreakTransform` (`SceneComponent.GetRelativeTransform` Gun)))
  (bind (_returnvalue_roll _returnvalue_pitch _returnvalue_yaw) (`KismetMathLibrary.BreakRotator` (`KismetMathLibrary.FindLookAtRotation` (`KismetMathLibrary.MakeVector` 0.0) (- (`KismetMathLibrary.InverseTransformLocation` (`self.GetTransform`) Target) _returnvalue_location))))
  (`SceneComponent.K2_SetRelativeRotation` Gun (`KismetMathLibrary.MakeRotator` (`KismetMathLibrary.ClampAngle` _returnvalue_roll) (`KismetMathLibrary.ClampAngle` _returnvalue_pitch -10.0 10.0) (`KismetMathLibrary.ClampAngle` _returnvalue_yaw 50.0 130.0)) false false))

(fn `FireGun`
  (params (Gun :type "StaticMeshComponent Object Reference"))
  (locals (GunLoc :type "StaticMeshComponent Object Reference"))
  (bind _gunloc (`local.GunLoc`))
  (bind (_returnvalue_location _returnvalue_rotation _returnvalue_scale) (`KismetMathLibrary.BreakTransform` (`SceneComponent.GetSocketTransform` (`local.GunLoc`) "Muzzle" "RTS_World")))
  (set `local.GunLoc` Gun)
  (`|SpawnActorFromClass` (`self.ProjectileToFire`) (`KismetMathLibrary.MakeTransform` _returnvalue_location (* _returnvalue_rotation (`KismetMathLibrary.RandomFloatInRange` 0.98 1.02)) _returnvalue_scale) "AlwaysSpawn" "OverrideRootScale" self (`KismetMathLibrary.MakeVector` (* (`self.ProjectileSpeed`) (`KismetMathLibrary.RandomFloatInRange` 0.98 1.02))) (`self.Instigator`) true)
  (`PrimitiveComponent.AddImpulseAtLocation` _gunloc (`KismetMathLibrary.TransformLocation` (`self.GetTransform`) (* (`KismetMathLibrary.GetForwardVector` (`SceneComponent.RelativeRotation` _gunloc)) -5000000.0)) (`SceneComponent.K2_GetComponentLocation` _gunloc) "None"))

(fn `UserConstructionScript`
  (bind _guns_collection (`self.Guns_Collection`))
  (`parent.UserConstructionScript`)
  (`KismetArrayLibrary.Array_Add` _guns_collection (`self.Gun_R01`))
  (`KismetArrayLibrary.Array_Add` _guns_collection (`self.Gun_R02`))
  (`KismetArrayLibrary.Array_Add` _guns_collection (`self.Gun_R03`))
  (`KismetArrayLibrary.Array_Add` _guns_collection (`self.Gun_R04`)))