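; Physics-driven snowmobile vehicle Blueprint with an animated spline track, scroll camera zoom and debug drawing.
; Construction sets center of mass, totals bone mass and lays instanced treads along the track spline.
; Throttle input picks a driving state that swaps the sprocket constraint profile, applies mass-scaled torque and switches brake and reverse lights.
; Sprocket rotation offsets treads along the spline; steering and drag are empty stubs.
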(event `InputAxis|MoveRight`
  (params (AxisValue :type "Float (single-precision)"))
  ;[1 1 1] Vehicle Movement Controls
  (`self.HandleSteering` AxisValue))

(event `InputAxis|MoveForward`
  (params (AxisValue :type "Float (single-precision)"))
  ;[1 1 1] Vehicle Movement Controls
  (`self.HandleDriving` AxisValue))

(event `self.Body.OnComponentHit`
  (params (HitComponent :type "PrimitiveComponent Object Reference") (OtherActor :type "Actor Object Reference") (OtherComp :type "PrimitiveComponent Object Reference") (NormalImpulse :type "Vector Structure") (Hit :type "HitResult Structure (by ref)"))
  ;[1 1 1] Process collision
  (if (`self.DebugMode`)
    (`KismetSystemLibrary.DrawDebugPoint` Hit_ImpactPoint 20.0 (struct :`R` 0.556863 :`B` 0.007843 :`A` 1.0) 5.0)))

(event `OnUserScrolled_Event`
  (params (CurrentOffset :type "Float (double-precision)"))
  (bind _springarm (`self.SpringArm`))
  (bind _targetarmlength (`SpringArmComponent.TargetArmLength` _springarm))
  ;[1 1 1] Camera Control
  (if (< 0.0 CurrentOffset)
    (set `SpringArmComponent.TargetArmLength` (+ _targetarmlength -25.0) _springarm)
    (else
      (set `SpringArmComponent.TargetArmLength` (+ _targetarmlength 25.0) _springarm))))

(event `self.ReceiveTick`
  (params (DeltaSeconds :type "Float (single-precision)"))
  (`self.Debug` DeltaSeconds)
  (`self.HandleLights`))

(event `Debug`
  (params (DeltaSeconds :type "Float (double-precision)"))
  (if (`self.DebugMode`)
    (`KismetSystemLibrary.PrintString` (`KismetStringLibrary.Conv_NameToString` (`self.DrivingState`)) true false (struct :`R` 1.0 :`G` 0.218246 :`B` 0.197917 :`A` 1.0) 0.0)))

(event `self.ReceiveBeginPlay`
  ;[1 1 1] Vehicle Debugging Mod
  (if (`self.DebugMode`)
    (`KismetSystemLibrary.ExecuteConsoleCommand` "pxvis collision")))

(event `self.F_L01.OnComponentHit`
  (params (HitComponent :type "PrimitiveComponent Object Reference") (OtherActor :type "Actor Object Reference") (OtherComp :type "PrimitiveComponent Object Reference") (NormalImpulse :type "Vector Structure") (Hit :type "HitResult Structure (by ref)")))

(fn `ApplyDrag`)

(fn `BuildTrackSpline`
  (returns (Dummy :type Boolean))
  (locals (SplineLoc :type "SplineComponent Object Reference") (TreadsLoc :type "InstancedStaticMeshComponent Object Reference"))
  (bind _trackspline (`self.TrackSpline`))
  (bind (_min _max) (`StaticMeshComponent.GetLocalBounds` (`self.Tread`)))
  (bind _returnvalue (`KismetMathLibrary.Abs` (- (.x _min) (.x _max))))
  (bind _returnvalue_2 (- _returnvalue 1.0))
  (bind _returnvalue_3 (`KismetMathLibrary.FCeil` (/ (`SplineComponent.GetSplineLength` _trackspline) _returnvalue_2)))
  (for _index (range (+ _returnvalue_3 1))
    (bind _returnvalue_4 (* _index _returnvalue))
    (bind (_returnvalue_roll _returnvalue_pitch _returnvalue_yaw) (`KismetMathLibrary.BreakRotator` (`SplineComponent.GetRotationAtDistanceAlongSpline` _trackspline _returnvalue_4 "Local")))
    (bind (_returnvalue_x _returnvalue_y) (`KismetMathLibrary.BreakVector` (`SplineComponent.GetRightVectorAtDistanceAlongSpline` _trackspline _returnvalue_4 "Local")))
    (`InstancedStaticMeshComponent.AddInstance` (`self.Tread`) (`KismetMathLibrary.MakeTransform` (`SplineComponent.GetLocationAtDistanceAlongSpline` _trackspline _returnvalue_4 "Local") (`KismetMathLibrary.MakeRotator` (`KismetMathLibrary.SelectFloat` 180.0 _returnvalue_roll (< _returnvalue_y 0.0)) _returnvalue_pitch _returnvalue_yaw))))
  (set `self.TreadLength` _returnvalue_2)
  (set `self.TreadsNumber` _returnvalue_3)
  (return false))

(fn `CalcTotalMass`
  (bind _snowmobile (`self.Snowmobile`))
  (for _array_element (`SceneComponent.GetAllSocketNames` _snowmobile)
    (set `self.TotalMass` (+ (`SkeletalMeshComponent.GetBoneMass` _snowmobile _array_element true) (`self.TotalMass`)))))

(fn `GetAcc`
  (returns (Acc :type "Float (double-precision)"))
  (return (* (* (`self.Acceleration`) -1000) (`self.TotalMass`))))

(fn `GetSpline`
  (params (Spline :type "SplineComponent Object Reference"))
  (returns (Points :type "Array of Vector Structure") (Tangens :type "Array of Vector Structure"))
  (bind _returnvalue (`SplineComponent.GetNumberOfSplinePoints` Spline))
  (bind _array (`|MakeArray`))
  (bind _array_2 (`|MakeArray`))
  (for _index (range (+ _returnvalue 1))
    (`KismetArrayLibrary.Array_Add` _array_2 (`SplineComponent.GetLocationAtSplinePoint` Spline _index "Local")))
  (for _index_2 (range (+ _returnvalue 1))
    (`KismetArrayLibrary.Array_Add` _array (`SplineComponent.GetTangentAtSplinePoint` Spline _index_2 "Local")))
  (return _array_2 _array))

(fn `HandleDriving`
  (params (AxisVal :type "Float (double-precision)"))
  (locals (WheelRotation :type "Float (double-precision)") (Reversing :type Boolean) (Acc :type "Float (double-precision)"))
  (bind _returnvalue (`KismetMathLibrary.NearlyEqual_FloatFloat` 0.0 AxisVal 0.01))
  (bind _returnvalue_2 (< AxisVal 0.0))
  (bind _sprocketname (`self.SprocketName`))
  (bind _snowmobile (`self.Snowmobile`))
  (bind _snowmobile_2 (`self.Snowmobile`))
  (bind _returnvalue_3 (`SplineComponent.GetSplineLength` (`self.TrackSpline`)))
  (bind _returnvalue_4 (`SceneComponent.GetSocketLocation` _snowmobile_2 _sprocketname))
  (bind _returnvalue_5 (`SceneComponent.K2_GetComponentLocation` _snowmobile))
  (bind _returnvalue_6 (`SceneComponent.GetComponentVelocity` _snowmobile))
  (bind _returnvalue_7 (`KismetMathLibrary.GetRightVector` (`SceneComponent.GetSocketRotation` _snowmobile_2 _sprocketname)))
  (bind _returnvalue_8 (`KismetMathLibrary.GetForwardVector` (`SceneComponent.K2_GetComponentRotation` _snowmobile)))
  (bind _returnvalue_9 (* _returnvalue_7 (* (`local.Acc`) AxisVal)))
  (bind _acc (`self.GetAcc`))
  (set `local.Acc` _acc)
  (`|ExecutionSequence`
    (:`then_0`
      (if _returnvalue
        (set `self.DrivingState` "Free")
        (if (and (< 1.0 (`KismetMathLibrary.VSize` (- _returnvalue_8 (`KismetMathLibrary.Normal` _returnvalue_6)))) (or _returnvalue_2 _returnvalue)) :!label _label
          (set `self.DrivingState` "Reverse"))
        (elif _returnvalue_2
          (set `self.DrivingState` "Brake")
          (goto _label)
          (else
            (set `self.DrivingState` "Drive")))))
    (:`then_2`
      (`SkeletalMeshComponent.SetConstraintProfile` (`self.Snowmobile`) (`self.SprocketName`) (`self.DrivingState`) true))
    (:`then_3`
      ;[1 1 1] Debug
      (if (`self.DebugMode`)
        (`KismetSystemLibrary.DrawDebugArrow` _returnvalue_4 (+ _returnvalue_4 _returnvalue_9) 100.0 (struct :`R` 1.0 :`G` 0.110692 :`A` 1.0) 0.0 4.0)
        (`KismetSystemLibrary.PrintString` (`KismetStringLibrary.Concat_StrStr` "Speed:" (`KismetStringLibrary.Conv_DoubleToString` (`KismetMathLibrary.VSize` (`self.GetVelocity`)))) true false (struct :`R` 0.324537 :`G` 1.0 :`A` 1.0) 0.0)
        (`KismetSystemLibrary.DrawDebugArrow` _returnvalue_5 (+ _returnvalue_5 _returnvalue_6) 100.0 (struct :`R` 0.115363 :`G` 1.0 :`A` 1.0) 0.0 4.0)
        (`KismetSystemLibrary.DrawDebugArrow` _returnvalue_5 (+ _returnvalue_5 (* _returnvalue_8 (400.0 400.0 400.0))) 100.0 (struct :`R` 0.60103 :`B` 1.0 :`A` 1.0) 0.0 4.0)))
    (:`then_4`
      ;[1 1 1] Animate track
      (if (> (.roll (`SceneComponent.GetSocketRotation` (`self.Snowmobile`) (`self.SprocketName`))) 90.0)
        (set `local.WheelRotation` 90.0)
        (else
          (set `local.WheelRotation` -270.0)))
      (for _index (range (+ (`self.TreadsNumber`) 1))
        (bind _returnvalue_10 (+ (* (`self.TreadLength`) (`KismetMathLibrary.Conv_IntToDouble` _index)) (* _returnvalue_3 (/ (`KismetMathLibrary.Abs` (- (`local.WheelRotation`) (.pitch (`SceneComponent.GetSocketRotation` (`self.Snowmobile`) (`self.SprocketName`))))) 360.0))))
        (bind _returnvalue_11 (`SplineComponent.GetTransformAtDistanceAlongSpline` (`self.TrackSpline`) (`KismetMathLibrary.SelectFloat` _returnvalue_10 (- _returnvalue_10 _returnvalue_3) (< _returnvalue_10 _returnvalue_3)) "Local" true))
        (bind _rotation (.rotation _returnvalue_11))
        (bind (_returnvalue_x _returnvalue_y) (`KismetMathLibrary.BreakVector` (`KismetMathLibrary.GetRightVector` _rotation)))
        (`InstancedStaticMeshComponent.UpdateInstanceTransform` (`self.Tread`) _index (`KismetMathLibrary.MakeTransform` (.location _returnvalue_11) (`KismetMathLibrary.TransformRotation` _returnvalue_11 (`KismetMathLibrary.MakeRotator` (`KismetMathLibrary.SelectFloat` 180.0 (.roll _rotation) (< _returnvalue_y 0.0)))) (.scale _returnvalue_11)) false true true)))
    (:`then_5`
      (switch `name` (`self.DrivingState`)
        (:`Drive`
          ;[1 1 1] Accelerate
          (`PrimitiveComponent.AddTorqueInDegrees` (`self.Snowmobile`) _returnvalue_9 (`self.SprocketName`) false))
        (:`Reverse`
          ;[1 1 1] Reverse
          (`PrimitiveComponent.AddTorqueInDegrees` (`self.Snowmobile`) (* _returnvalue_7 (* (`local.Acc`) AxisVal)) (`self.SprocketName`) false))))))

(fn `HandleLights`
  (bind _brakelight (`self.BrakeLight`))
  (bind _reverselight (`self.ReverseLight`))
  (switch `name` (`self.DrivingState`)
    (:`Free`
      (`|ExecutionSequence`
        (:`then_0`
          (`/Engine/EditorBlueprintResources/StandardMacros.Gate` false :!label _label
            (:`Exit`
              (`LightComponent.SetIntensity` _reverselight 1500.0))))
        (:`then_1`
          (`/Engine/EditorBlueprintResources/StandardMacros.Gate` false :!label _label_2
            (:`Exit`
              (`LightComponent.SetIntensity` _reverselight 0.0))))
        (:`then_2`
          (`/Engine/EditorBlueprintResources/StandardMacros.Gate` false :!label _label_3
            (:`Exit`
              (`LightComponent.SetIntensity` _brakelight 300.0))))))
    (:`Drive`
      (`|ExecutionSequence`
        (:`then_0`
          (goto _label :!via `Close`))
        (:`then_1`
          (goto _label_2))
        (:`then_2`
          (goto _label_2 :!via `Open`))
        (:`then_3`
          (goto _label_3))))
    (:`Brake`
      (`|ExecutionSequence`
        (:`then_0`
          (`/Engine/EditorBlueprintResources/StandardMacros.Gate` false :!label _label_4
            (:`Exit`
              (`LightComponent.SetIntensity` _brakelight 1500.0))))
        (:`then_1`
          (goto _label_4 :!via `Open`))))
    (:`Reverse`
      (`|ExecutionSequence`
        (:`then_0`
          (goto _label :!via `Open`))
        (:`then_1`
          (goto _label))
        (:`then_2`
          (goto _label_4 :!via `Close`))))))

(fn `HandleSteering`
  (params (AxisVal :type "Float (double-precision)")))

(fn `SetCOM`
  (bind _snowmobile (`self.Snowmobile`))
  (`PrimitiveComponent.SetCenterOfMass` _snowmobile (-40.0 10.0 0.0) "Body")
  (`SceneComponent.K2_SetWorldLocation` (`self.COM`) (`PrimitiveComponent.GetCenterOfMass` _snowmobile "None") false true))

(fn `UserConstructionScript`
  (`|ExecutionSequence`
    (:`then_0`
      (`self.SetCOM`))
    (:`then_1`
      (`self.BuildTrackSpline`)
      (`InstancedStaticMeshComponent.RemoveInstance` (`self.Tread`) 0))
    (:`then_3`
      (`self.CalcTotalMass`))))