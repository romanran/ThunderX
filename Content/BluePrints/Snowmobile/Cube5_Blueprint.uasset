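; Test physics cube Blueprint in the Snowmobile folder that pushes its static mesh along world X against velocity-based drag.
; Each Tick it applies a force equal to the negated velocity plus a small constant +X push, so motion tends toward a steady low speed.
; It prints the current speed to the screen every frame for debugging.
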(event `self.ReceiveTick`
  (params (DeltaSeconds :type "Float (single-precision)"))
  (bind _staticmeshcomponent (`self.StaticMeshComponent`))
  (bind _returnvalue (`SceneComponent.GetComponentVelocity` _staticmeshcomponent))
  (`PrimitiveComponent.AddForce` _staticmeshcomponent (- (`KismetMathLibrary.NegateVector` _returnvalue) (-10.0 0.0 0.0)) "None" false)
  (`KismetSystemLibrary.PrintString` (`KismetStringLibrary.Conv_DoubleToString` (`KismetMathLibrary.VSize` _returnvalue)) true false (struct :`G` 0.66 :`B` 1.0 :`A` 1.0) 0.0))

(event `self.ReceiveBeginPlay`)

(fn `UserConstructionScript`)