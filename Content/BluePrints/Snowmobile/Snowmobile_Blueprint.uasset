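; Snowmobile Blueprint, a child class that handles the vehicle's track spline and tread animation.
; Construction and track-spline building defer to the parent class.
; AnimateTrack reads the spline points and calls the control-point animation with the suspension setup once per point, passing the whole array each time.
; The instanced-mesh tread animation is left disconnected, and the event graph holds only disabled stub events.
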(fn `AnimateTrack`
  (bind _points (`self.GetSpline` (`self.TrackSpline`)))
  (for _array_element _points
    (`self.AnimateTreadsSplineControlPoints` null (`self.TrackSpline`) 0 0 _points (`self.SuspesionSetup`))))

(fn `BuildTrackSpline`
  (params (TrackSpline :type "SplineComponent Object Reference") (TreadModel :type "InstancedStaticMeshComponent Object Reference"))
  (returns (Dummy :type Boolean))
  (bind _dummy (`parent.BuildTrackSpline` (`self.TrackSpline`) (`self.TreadModel`)))
  (return _dummy))

(fn `UserConstructionScript`
  (`parent.UserConstructionScript`))