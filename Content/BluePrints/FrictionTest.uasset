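; Test actor that experiments with custom ground friction on a physics-simulated static mesh using MMT physics functions.
; On each MMT physics tick, a tiny box trace runs a short way down along Corner1's local down axis.
; On a hit, AddFriction applies a force at the impact point opposing the mesh's point velocity, scaled by its mass, and draws it as a debug arrow.
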(event `self.MMTPhysicsTick`
  (params (SubstepDeltaTime :type "Float (single-precision)"))
  (bind _returnvalue (`MMTBPFunctionLibrary.MMTGetTransformComponent` (`self.Corner1`)))
  (bind (_outhit _returnvalue_2) (`KismetSystemLibrary.BoxTraceSingle` :`Start` (.location _returnvalue) :`End` (+ (.location _returnvalue) (* (`KismetMathLibrary.GetUpVector` (.rotation _returnvalue)) -1.0)) :`HalfSize` (0.1 0.1 0.0) :`TraceChannel` "TraceTypeQuery1" :`TraceColor` (struct :`R` 0.510417 :`G` 0.055992 :`A` 1.0) :`TraceHitColor` (struct :`R` 0.520833 :`G` 0.271241 :`A` 1.0) :`DrawTime` 1.0))
  (if _returnvalue_2
    (`self.AddFriction` _outhit)))

(fn `AddFriction`
  (params (Hit :type "HitResult Structure"))
  (locals (ImpactPoint :type "Vector Structure") (Upnormal :type "Vector Structure") (TerrainFriction :type "Float (double-precision)"))
  (bind _impactpoint (`local.ImpactPoint`))
  (`MMTBPFunctionLibrary.MMTGetTransformComponent` (`self.StaticMesh`))
  (set `local.ImpactPoint` (`.ImpactPoint` (`GameplayStatics.BreakHitResult` Hit)))
  (bind _returnvalue (`PrimitiveComponent.GetPhysicsLinearVelocityAtPoint` (`self.StaticMesh`) (`local.ImpactPoint`) "None"))
  (bind _returnvalue_2 (* (`KismetMathLibrary.NegateVector` _returnvalue) (`PrimitiveComponent.GetMass` (`self.StaticMesh`))))
  (`MMTBPFunctionLibrary.MMTAddForceAtLocationComponent` (`self.StaticMesh`) _returnvalue_2 _impactpoint)
  (`KismetSystemLibrary.DrawDebugArrow` _impactpoint (+ _impactpoint (* _returnvalue_2 0.1)) 2.0 (struct :`G` 1.0 :`B` 0.55007 :`A` 1.0) 0.0 1.0))

(fn `UserConstructionScript`)